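; Key pickup platform that lets the player collect a key by interacting with the statue on it.
; A Box trigger enables the actor's input while the player character overlaps it and disables it on exit.
; The interact action destroys the SMStatue component, increments NumberOfKeys on PlayerCharacter and plays a pitched-down pickup sound.
; The validity check on the statue keeps the key from being collected twice.
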(event `self.Box.OnComponentBeginOverlap`
  (params (OverlappedComponent :type "PrimitiveComponent Object Reference") (OtherActor :type "Actor Object Reference") (OtherComp :type "PrimitiveComponent Object Reference") (OtherBodyIndex :type Integer) (bFromSweep :type Boolean) (SweepResult :type "HitResult Structure (by ref)"))
  (if (== OtherActor (`GameplayStatics.GetPlayerCharacter` 0))
    (`self.EnableInput` (`GameplayStatics.GetPlayerController` 0))))

(event `InputAction|interact`
  (params (Key :type "Key Structure"))
  (bind _sm_statue (`self.SM_Statue`))
  (:`Pressed`
    (`/Engine/EditorBlueprintResources/StandardMacros.IsValid` _sm_statue
      (:`Is Valid`
        (`ActorComponent.K2_DestroyComponent` _sm_statue)
        (bind _asplayer_character (cast `/Game/PlayerCharacter` (`GameplayStatics.GetPlayerCharacter` 0)))
        (`/Engine/EditorBlueprintResources/StandardMacros.IncrementInt` (`/Game/PlayerCharacter.Number of Keys` _asplayer_character)
          (:`  `
            (`GameplayStatics.PlaySoundAtLocation` "/Game/PickupKey_SFX.PickupKey_SFX" (`self.K2_GetActorLocation` (`GameplayStatics.GetPlayerCharacter` 0)) (struct) 1.0 0.5 0.0 null null null null)))))))

(event `self.Box.OnComponentEndOverlap`
  (params (OverlappedComponent :type "PrimitiveComponent Object Reference") (OtherActor :type "Actor Object Reference") (OtherComp :type "PrimitiveComponent Object Reference") (OtherBodyIndex :type Integer))
  (if (== OtherActor (`GameplayStatics.GetPlayerCharacter` 0))
    (`self.DisableInput` (`GameplayStatics.GetPlayerController` 0))))

(fn `UserConstructionScript`)